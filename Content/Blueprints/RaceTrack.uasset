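; Race track actor that builds a track mesh and two parallel lane splines from an editable base spline in its construction script.
; It lays scaled spline mesh segments along BaseSpline, then rebuilds RaceTrack1 and RaceTrack2 by offsetting its points along their right vectors to either side.
; Lane tangents are copied from the base and shrunk or stretched by comparing point-to-point distances to compensate for curves.
; The event graph holds only unused logic.
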(event `self.ReceiveBeginPlay`)

(fn `CalculcateTangentCorrection`
  (params (Index :type Integer) (Spline :type "SplineComponent Object Reference"))
  (returns (CurveCorrection :type "Float (double-precision)"))
  (bind _basespline (`self.BaseSpline`))
  (if (> (`KismetMathLibrary.VSize` (- (`SplineComponent.GetLocationAtSplinePoint` _basespline Index "Local") (`SplineComponent.GetLocationAtSplinePoint` _basespline (- Index 1) "Local"))) (`KismetMathLibrary.VSize` (- (`SplineComponent.GetLocationAtSplinePoint` Spline Index "Local") (`SplineComponent.GetLocationAtSplinePoint` Spline (- Index 1) "Local"))))
    (return 0.9)
    (else
      (return 1.2))))

(fn `CreateRaceTrack`
  (params (RaceTrack :type "SplineComponent Object Reference") (Offset :type "Float (double-precision)"))
  (locals (NewLocalVar_0 :type String :default "Hello"))
  (bind _basespline (`self.BaseSpline`))
  (`|ExecutionSequence`
    (:`then_0`
      (`SplineComponent.ClearSplinePoints` RaceTrack true)
      (for _index (range (`self.GetNumberOfSplinePoints`))
        (`SplineComponent.AddSplinePoint` RaceTrack (+ (* (`KismetMathLibrary.Normal` (`SplineComponent.GetRightVectorAtSplinePoint` _basespline _index "Local")) Offset) (`SplineComponent.GetLocationAtSplinePoint` _basespline _index "Local")) "Local" true)))
    (:`then_1`
      (for _index_2 (range 1 (`self.GetNumberOfSplinePoints`))
        (bind _curvecorrection (`self.CalculcateTangentCorrection` _index_2 RaceTrack))
        (bind _curvecorrection_2 (`self.CalculcateTangentCorrection` (+ _index_2 1)))
        (bind _returnvalue (`SplineComponent.GetTangentAtSplinePoint` (`self.BaseSpline`) _index_2 "Local"))
        (`SplineComponent.SetTangentsAtSplinePoint` RaceTrack _index_2 (* _returnvalue _curvecorrection) (* _returnvalue _curvecorrection_2) "Local" true)))))

(fn `UserConstructionScript`
  (bind _basespline (`self.BaseSpline`))
  (for _index (range (+ (- (`self.GetNumberOfSplinePoints`) 2) 1))
    (bind _returnvalue (`AddComponent|NODE_AddSplineMeshComponent-0`))
    (bind _returnvalue_2 (+ _index 1))
    (`SplineMeshComponent.SetStartAndEnd` _returnvalue (`SplineComponent.GetLocationAtSplinePoint` _basespline _index "Local") (`SplineComponent.GetTangentAtSplinePoint` _basespline _index "Local") (`SplineComponent.GetLocationAtSplinePoint` _basespline _returnvalue_2 "Local") (`SplineComponent.GetTangentAtSplinePoint` _basespline _returnvalue_2 "Local") true)
    (`SplineMeshComponent.SetEndScale` _returnvalue (0.4 0.4) true)
    (`SplineMeshComponent.SetStartScale` _returnvalue (0.4 0.4) true))
  (`self.CreateRaceTrack` (`self.RaceTrack1`) 30.0)
  (`self.CreateRaceTrack` (`self.RaceTrack2`) -30.0))