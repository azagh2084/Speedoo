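; RaceCar is a player-controlled car that rides along a RaceTrack spline, looping back to the start at the end.
; Each Tick adds Speed to a spline distance and places the Cube at that transform, without delta-time scaling.
; Holding R accelerates; otherwise speed decays, clamped at zero.
; The F brake never engages because both press and release set IsDecelerating false.
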(event `self.ReceiveBeginPlay`
  ;[1 1 1] Begin Play
  (`self.EnableInput` (`GameplayStatics.GetPlayerController` 0))
  (set `self.RaceSpline` (`/Game/Blueprints/RaceTrack.Spline` (`self.RaceTrack`))))

(event `self.ReceiveTick`
  (params (DeltaSeconds :type "Float (single-precision)"))
  (`|ExecutionSequence`
    (:`then_0`
      (bind _output_get (set `self.Position` (+ (`self.Position`) (`self.Speed`) 0.0)))
      (`self.CheckPosition`)
      (bind (_returnvalue_location _returnvalue_rotation) (`KismetMathLibrary.BreakTransform` (`SplineComponent.GetTransformAtDistanceAlongSpline` (`self.RaceSpline`) _output_get "World" false)))
      (`SceneComponent.K2_SetWorldTransform` (`self.Cube`) (`KismetMathLibrary.MakeTransform` _returnvalue_location _returnvalue_rotation (0.2 0.2 0.2)) false false))
    (:`then_1`
      (if (`self.IsAccelerating`)
        (`self.AddSpeed` 0.3)
        (else
          (`self.AddSpeed` -0.2)
          (if (`self.IsDecelerating`)
            (`self.AddSpeed` -0.3))
          (`self.CheckSpeedZero`))))))

(event `CheckPosition`
  (if (>= (`self.Position`) (`SplineComponent.GetSplineLength` (`self.RaceSpline`)))
    (set `self.Position` 0.0)))

(event `CheckSpeed`)

(event `Key|R`
  (params (Key :type "Key Structure"))
  (:`Pressed`
    (set `self.IsAccelerating` true))
  (:`Released`
    (set `self.IsAccelerating` false)))

(event `Key|F`
  (params (Key :type "Key Structure"))
  (:`Pressed`
    (set `self.IsDecelerating` false))
  (:`Released`
    (set `self.IsDecelerating` false)))

(fn `UserConstructionScript`)